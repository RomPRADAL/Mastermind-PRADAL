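; BP_MastermindGM runs the answer feedback and win state for a Mastermind game.
; SpawnNewAnswer checks the good-place count: four triggers Win, otherwise it prints both counts and adds an answer display.
; Each new answer shifts earlier BP_ShowAnswer actors along X, then spawns at a fixed transform with both counts.
; Win destroys all answer actors, prints a message and spawns three Niagara celebration effects.
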(event EventSpawnNewAnswer
  (params (GoodPlace :type Integer) (WrongPlace :type Integer))
  (if (== GoodPlace 4)
    (CallFunction|Win)
    (else
      (Development|PrintString (Utilities|String|Append "Good place : " (Utilities|String|ToString(Integer) GoodPlace) ", Wrong place : " (Utilities|String|ToString(Integer) WrongPlace)))
      (CallFunction|SpawnNewAnswerOLD GoodPlace WrongPlace))))

(fn ConstructionScript)

(fn SpawnNewAnswerOLD
  (params (GoodPlace :type Integer) (WrongPlace :type Integer))
  (Utilities|FlowControl|Sequence
    (:then_0
      (for _array_element (Variables|Default|GetAllAnswer)
        (Transformation|SetActorLocation _array_element (Math|Vector|MakeVector (+ (.X (Math|Vector|BreakVector (Transformation|GetActorLocation _array_element))) (Variables|Default|GetOffsetValue)) (.Y (Math|Vector|BreakVector (Transformation|GetActorLocation _array_element))) (.Z (Math|Vector|BreakVector (Transformation|GetActorLocation _array_element)))) false false)))
    (:then_1
      (bind _returnvalue (Game|SpawnActorfromClass "/Game/Mastermind/Blueprints/BP_ShowAnswer.BP_ShowAnswer_C" (Variables|Default|GetAnswerSpawnLocation) "AdjustIfPossibleButAlwaysSpawn" "MultiplyWithRoot" 0 0))
      (Variables|/Game/Mastermind/Blueprints/BP_ShowAnswer.BP_ShowAnswer_C|SetGoodPlace _returnvalue GoodPlace)
      (Variables|/Game/Mastermind/Blueprints/BP_ShowAnswer.BP_ShowAnswer_C|SetWrongPlace _returnvalue WrongPlace)
      (Utilities|Array|AddUnique (Variables|Default|GetAllAnswer) _returnvalue))))

(fn AddOffsettoSpawnNewAnswer
  (params (Offsetvalue :type Float%20%28double-precision%29))
  (Variables|Default|SetAnswerSpawnLocation (Math|Transform|MakeTransform (Math|Vector|MakeVector (+ Offsetvalue (.X (Math|Vector|BreakVector (.Location (Math|Transform|BreakTransform (Variables|Default|GetAnswerSpawnLocation)))))) (.Y (Math|Vector|BreakVector (.Location (Math|Transform|BreakTransform (Variables|Default|GetAnswerSpawnLocation))))) (.Z (Math|Vector|BreakVector (.Location (Math|Transform|BreakTransform (Variables|Default|GetAnswerSpawnLocation)))))) (.Rotation (Math|Transform|BreakTransform (Variables|Default|GetAnswerSpawnLocation))) (.Scale (Math|Transform|BreakTransform (Variables|Default|GetAnswerSpawnLocation))))))

(fn Win
  (Utilities|FlowControl|Sequence
    (:then_0
      (for _array_element (Variables|Default|GetAllAnswer)
        (Actor|DestroyActor _array_element))
      (Development|PrintString "Win"))
    (:then_1
      (Niagara|SpawnSystematLocation "/Game/Mastermind/Blueprints/Niagara_GG.Niagara_GG" "-1350.000000,-550.000000,0.000000")
      (Niagara|SpawnSystematLocation "/Game/Mastermind/Blueprints/Niagara_GG.Niagara_GG" "-1450.000000,-550.000000,0.000000")
      (Niagara|SpawnSystematLocation "/Game/Mastermind/Blueprints/Niagara_GG.Niagara_GG" "-1250.000000,-550.000000,0.000000"))))